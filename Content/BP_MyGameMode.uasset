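; Game mode for a multiplayer hunter game that holds the match until the lobby is full, then picks a random Hunter.
; On PostLogin it spawns a BP_ThirdPersonCharacter at a PlayerStart and possesses it with the new controller.
; The ReadyToStartMatch override requires the player count to equal MAXPLAYERS.
; When OnSetMatchState sees the match started, it sets IsHunter on a random PlayerState from the game state's PlayerArray.
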(event `self.K2_PostLogin`
  (params (NewPlayer :type "PlayerController Object Reference"))
  ;[0 0 0] a chaque nouvelle connexion on spawn un Character et on le possess
  (`parent.K2_PostLogin` NewPlayer)
  (bind _returnvalue (`GameplayStatics.GetActorOfClass` "/Script/Engine.PlayerStart"))
  (bind _returnvalue_2 (`|SpawnActorFromClass` "/Game/BP_ThirdPersonCharacter.BP_ThirdPersonCharacter_C" (`self.GetTransform` _returnvalue) "AdjustIfPossibleButAlwaysSpawn" "MultiplyWithRoot" null null))
  (`Controller.Possess` NewPlayer _returnvalue_2))

(event `self.K2_OnSetMatchState`
  (params (NewState :type Name))
  (bind _returnvalue (`self.HasMatchStarted`))
  (`parent.K2_OnSetMatchState` NewState)
  (`KismetSystemLibrary.PrintString` (`KismetStringLibrary.Concat_StrStr` (`KismetStringLibrary.Conv_NameToString` NewState) "=> " (`KismetStringLibrary.Conv_BoolToString` _returnvalue)) true false)
  (if _returnvalue
    ;[0 0 0] ici le server choisit le Hunter (on pourrait deplacer cette partie dans une fonction de GameState)
    (bind _asbp_my_game_state (cast `/Game/BP_MyGameState` (`GameplayStatics.GetGameState`)))
    (bind _asbp_my_player_state (cast `/Game/BP_MyPlayerState` (`KismetArrayLibrary.Array_Random` (`GameStateBase.PlayerArray` _asbp_my_game_state))))
    (set `/Game/BP_MyPlayerState.bIsHunter` true _asbp_my_player_state)))

(fn `ReadyToStartMatch`
  (returns (ReturnValue :type Boolean))
  (bind _returnvalue (`parent.ReadyToStartMatch`))
  (bind _returnvalue_2 (`self.GetNumPlayers`))
  (return (and _returnvalue (== _returnvalue_2 (`self.MAX_PLAYERS`)))))

(fn `UserConstructionScript`)